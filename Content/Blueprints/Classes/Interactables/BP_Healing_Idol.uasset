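; BP_Healing_Idol is an interactable idol that heals the player when used.
; Its InteractwithObject event calls the healing function, then prints a "Healed" message.
; The function adds the Healing amount directly to CurrentHealth on the BPC_Combat component of player character 0, ignoring the interactor and applying no clamp.
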(event `self.Interact_With_Object`
  (params (Hit_Results :type "HitResult Structure") (Intoractor :type "Actor Object Reference"))
  (`self.Healing_Idol`)
  (`KismetSystemLibrary.PrintString` "Healed"))

(fn `UserConstructionScript`
  (`parent.UserConstructionScript`))