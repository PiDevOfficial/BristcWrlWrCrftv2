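; BPC_AiPatrol is an AI patrol component that supplies the next location along a list of patrol point actors.
; FindNextPoint takes the actor at the current index, steps the index, and returns that actor's location if valid.
; The FlipedPath flag reverses the step direction at the first and last points, so the route ping-pongs instead of looping.
; It has no active events and works only when called.
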(fn `FindNextPoint`
  (returns (Location :type "Vector Structure"))
  (locals (LocalPoint :type "Actor Object Reference"))
  (bind _patrolpoints (`self.PatrolPoints`))
  (set `local.LocalPoint` (`|GetArrayItem` (`self.PatrolPoints`) (`self.CurrentPoint`)))
  (if (`self.FlipedPath?`)
    (set `self.CurrentPoint` (- (`self.CurrentPoint`) 1))
    (if (== (`self.CurrentPoint`) (`KismetArrayLibrary.Array_Find` _patrolpoints (`|GetArrayItem` _patrolpoints)))
      (set `self.FlipedPath?` false)
      (else
        (set `self.FlipedPath?` true)))
    (else
      (set `self.CurrentPoint` (+ (`self.CurrentPoint`) 1))
      (set `self.FlipedPath?` (== (`self.CurrentPoint`) (`KismetArrayLibrary.Array_LastIndex` (`self.PatrolPoints`))))))
  (bind _localpoint (`local.LocalPoint`)
    (:`then`
      (return (`Actor.K2_GetActorLocation` _localpoint)))
    (:`else`)))