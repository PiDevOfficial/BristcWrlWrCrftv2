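; BPC_Movement is an AI movement component that sets its owning character's walk speed from a movement mode.
; SetMovementMode stores the given mode and maps Walking, Running or Sprinting to its configured speed, writing it to the CharacterMovementComponent's MaxWalkSpeed.
; BeginPlay applies the current MovementMode so the owner starts at the matching speed.
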(event `self.ReceiveBeginPlay`
  (`self.SetMovementMode` (`self.MovementMode`)))

(event `SetMovementMode`
  (params (NewParam :type "/Game/AdvancedLocomotionV4/Data/Enums/ALS_Gait Enum" :default "NewEnumerator0"))
  (set `self.MovementMode` NewParam)
  (set `CharacterMovementComponent.MaxWalkSpeed` (select `/Game/AdvancedLocomotionV4/Data/Enums/ALS_Gait` NewParam :`NewEnumerator0` (`self.WalkingSpeed`) :`NewEnumerator1` (`self.RunningSpeed`) :`NewEnumerator2` (`self.SprintingSpeed`) :!type "Float (single-precision)") (`Actor.GetComponentByClass` (`self.GetOwner`) "/Script/Engine.CharacterMovementComponent")))