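; BPC_Interact is an interaction component that detects whether the player character faces something it could interact with.
; Pressing the Interact input passes player 0's character to InteractCheck, which sphere-traces the Visibility channel forward from the actor's location over InteractDistance.
; A hit sets CanInteract and stores HitResults, while a miss only clears CanInteract.
; The file performs no interaction on the hit object itself.
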(event `InputAction|Interact`
  (params (Key :type "Key Structure"))
  ;[1 1 1] Gets character and checks if object can be interacted with
  (:`Pressed`
    (`self.Interact_Check` (`GameplayStatics.GetPlayerCharacter` 0))))

(fn `Interact_Check`
  (params (Get_Pawn_Data :type "Pawn Object Reference"))
  (bind _returnvalue (`Actor.K2_GetActorLocation` Get_Pawn_Data))
  (bind (_outhit _returnvalue_2) (`KismetSystemLibrary.SphereTraceSingle` _returnvalue (+ _returnvalue (* (`Actor.GetActorForwardVector` Get_Pawn_Data) (`self.Interact_Distance`))) 40.0 "TraceTypeQuery1"))
  (if _returnvalue_2
    (set `self.Can_interact` true)
    (set `self.Hit_Results` _outhit)
    (else
      (set `self.Can_interact` false))))