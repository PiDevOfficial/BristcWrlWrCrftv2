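; Actor component that lets the player interact with objects in front of their character.
; On the Interact input press, it sphere-traces on the Visibility channel from the player character along its forward vector up to InteractDistance, with debug drawing enabled.
; A hit actor that casts to BP_Master_Interact receives InteractWithObject with the hit result and the interacting character, leaving the response to that class.
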(event `InputAction|Interact`
  (params (Key :type "Key Structure"))
  ;[1 1 1] checks if object can be interacted with
  (:`Pressed`
    (`self.Interact_Check` (`GameplayStatics.GetPlayerCharacter` 0))))

(fn `Interact_Check`
  (params (Get_Pawn_Data :type "Pawn Object Reference"))
  (bind _returnvalue (`Actor.K2_GetActorLocation` Get_Pawn_Data))
  (bind (_outhit _returnvalue_2) (`KismetSystemLibrary.SphereTraceSingle` :`Start` _returnvalue :`End` (+ _returnvalue (* (`Actor.GetActorForwardVector` Get_Pawn_Data) (`self.Interact_Distance`))) :`Radius` 40.0 :`TraceChannel` "TraceTypeQuery1" :`DrawDebugType` "ForDuration"))
  (if _returnvalue_2
    (bind _asbp_master_interact (cast `/Game/Blueprints/Libraries/BP_Master_Interact` (`.HitActor` (`GameplayStatics.BreakHitResult` _outhit))))
    (`/Game/Blueprints/Libraries/BP_Master_Interact.Interact_With_Object` _asbp_master_interact _outhit Get_Pawn_Data)))