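; Inventory component that toggles the inventory screen from the ShowInventory input action.
; A FlipFlop alternates calls to ShowInventory, which creates a fresh UI_Inventory widget, adds it to the viewport and refreshes it, or removes the existing one.
; The live path is commented as old inventory code, while an equipment menu variant sits disconnected and never runs.
; It holds no item logic: InventoryItems is unused and the custom event is empty.
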(event `InputAction|ShowInventory`
  (params (Key :type "Key Structure"))
  ;[1 1 1] Show Inventory
  (:`Pressed`
    (`/Engine/EditorBlueprintResources/StandardMacros.FlipFlop`
      (:`A`
        (`self.ShowInventory` true))
      (:`B`
        (`self.ShowInventory` false)))))

(event `CustomEvent_0`)

(fn `ShowInventory`
  (params (`Show?` :type Boolean))
  ;[1 1 1] OId Inventory Code
  (if `Show?`
    (bind _returnvalue (`|CreateWidget` "/Game/UI/Widgets/Inventory/UI_Inventory.UI_Inventory_C"))
    (bind _output_get (set `self.InventoryWidget` _returnvalue))
    (`UserWidget.AddToViewport` _output_get 0)
    (`/Game/UI/Widgets/Inventory/UI_Inventory.UpdateInventory` _output_get)
    (else
      (bind _inventorywidget (`self.InventoryWidget`)
        (:`then`
          (`Widget.RemoveFromParent` _inventorywidget))
        (:`else`)))))