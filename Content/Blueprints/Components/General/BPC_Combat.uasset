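; BPC_Combat is a reusable character combat component handling weapon equipping, attacks, rolling, stamina, damage, death and team checks.
; Light, thrust and dive attack montages are gated by state and stamina, with combos picked by overlay state and counter, and "CanAttack" notifies reopening input.
; Hits scale damage by attacker ATK over DEF, with optional time-dilation hit freeze and camera shake; death awards orbs to the killer.
; It also toggles the level-up menu.
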(event `self.ReceiveTick`
  (params (DeltaSeconds :type "Float (single-precision)"))
  ;[1 1 1] Tick
  (if (< (`self.CurrentStamina`) (`self.MaxStamina`))
    (if (not (`self.IsAttacking`))
      (set `self.CurrentStamina` (`KismetMathLibrary.FClamp` (+ (`self.CurrentStamina`) (`self.StaminaRegenSpeed`)) 0.0 (`self.MaxStamina`))))))

(event `Initialization`
  (params (SkeletalMesh :type "SkeletalMeshComponent Object Reference") (WeaponMesh :type "StaticMeshComponent Object Reference") (CapsuleComp :type "CapsuleComponent Object Reference"))
  ;[1 1 1] Initialization
  (set `self.Skeletal Mesh` SkeletalMesh)
  (set `self.Weapon Mesh` WeaponMesh)
  (set `self.Capsule Comp` CapsuleComp))

(event `EquipWeapon`
  (params (`Draw Weapon?` :type Boolean))
  ;[1 1 1] EquipWeapon
  (if `Draw Weapon?`
    (bind _notifyname (`|PlayMontage` (`self.Skeletal Mesh`) (`self.GetEquipAnimation`))
      (:`OnNotifyBegin`
        (if (== _notifyname "EquipWeapon")
          (`SceneComponent.K2_AttachToComponent` (`self.Weapon Mesh`) (`self.Skeletal Mesh`) (`self.Hand Socket`) "KeepRelative" "KeepRelative" "KeepRelative" true)
          (message `/Game/AdvancedLocomotionV4/Blueprints/Interfaces/ALS_Character_BPI.BPI_Set_OverlayState` (`self.GetOwner`) (`self.Overlay State`))
          (set `self.IsCombat?` true))))
    (else
      (set `self.IsCombat?` true))))

(event `InputAction|EquipWeapon`
  (params (Key :type "Key Structure"))
  ;[1 1 1] EquipWeapon
  (:`Pressed`
    (`self.EquipWeapon` true)))

(event `LightAttack`
  ;[1 1 1] Attacks
  ;;[1 1 1] Light Attack
  (`self.Can Attack Check`)
  (bind _notifyname (`|PlayMontage` (`self.Skeletal Mesh`) (`self.GetLightAttackAnimation`))
    (:`then`
      (`/Engine/EditorBlueprintResources/StandardMacros.IncrementInt` (`self.LightAttackComboCount`)
        (:`  `
          (set `self.IsAttacking` true)
          (`self.ReduceStamina` 15.0)
          (`self.Rotation Correction`))))
    (:`OnInterrupted`
      (set `self.IsAttacking` false :!label _label))
    (:`OnNotifyBegin`
      (if (== _notifyname "CanAttack")
        (goto _label)))))

(event `Die`
  (params (Attacker :type "Actor Object Reference"))
  (bind _returnvalue (`Actor.GetComponentByClass` Attacker "BPC_Combat_C"))
  ;[1 1 1] Die & Get hit
  (set `/Game/Blueprints/Components/General/BPC_Combat.CurrentOrbs` (+ (`/Game/Blueprints/Components/General/BPC_Combat.CurrentOrbs` _returnvalue) (`self.OrbsRewardOnDeath`)) _returnvalue)
  (`self.ResetTimeDilation`)
  (`Actor.K2_DestroyActor` (`self.GetOwner`)))

(event `InputAction|Ability Slot 1`
  (params (Key :type "Key Structure"))
  ;[1 1 1] Attacks
  ;;[1 1 1] Light Attack
  (:`Pressed`
    (`self.LightAttack`)))

(event `GetHit`
  (params (Attacker :type "Actor Object Reference") (`FrameFreeze?` :type Boolean) (DamageMultiplayer :type "Float (double-precision)" :default 1.0))
  ;[1 1 1] Die & Get hit
  (`self.GetHitCheck`)
  (set `self.CanGetHit` false)
  (`self.DamageCaluculation` Attacker DamageMultiplayer)
  (`self.DamageEffects` `FrameFreeze?` Attacker)
  (`GameplayStatics.ApplyDamage` (`self.GetOwner`) 1.0 null Attacker)
  (`self.DeathCheck` Attacker)
  (`KismetSystemLibrary.Delay` 0.2)
  (set `self.CanGetHit` true))

(event `ThrustAttack`
  ;[1 1 1] Attacks
  ;;[1 1 1] Thrust Attack
  (`self.Can Attack Check`)
  (bind _notifyname (`|PlayMontage` (`self.Skeletal Mesh`) (`self.Get ThrustAttack Animation`))
    (:`then`
      (`/Engine/EditorBlueprintResources/StandardMacros.IncrementInt` (`self.ThrustAttackComboCount`)
        (:`  `
          (set `self.IsAttacking` true)
          (`self.ReduceStamina` 15.0)
          (`self.Rotation Correction`))))
    (:`OnInterrupted`
      (set `self.IsAttacking` false :!label _label_2))
    (:`OnNotifyBegin`
      (if (== _notifyname "CanAttack")
        (goto _label_2)))))

(event `Roll`
  (bind _returnvalue (`self.GetOwner`))
  ;[1 1 1] Roll
  (`self.RollCheck`)
  (bind _newparam (message `/Game/Blueprints/Libraries/BPI_Inventory.GetLastMovementDirection` _returnvalue))
  (`Actor.K2_SetActorRotation` _returnvalue (`KismetMathLibrary.Conv_VectorToRotator` _newparam) false)
  (`|PlayMontage` (`self.Skeletal Mesh`) "/Game/Animations/SwordnShield/Mannequin_RM/Roll_f.Roll_f"
    (:`then`
      (set `self.IsRolling?` true))
    (:`OnBlendOut`
      (set `self.IsRolling?` false :!label _label_3))
    (:`OnInterrupted`
      (goto _label_3))))

(event `InputAction|Ability Slot 2`
  (params (Key :type "Key Structure"))
  ;[1 1 1] Attacks
  ;;[1 1 1] Thrust Attack
  (:`Pressed`
    (`self.ThrustAttack`)))

(event `InputAction|AbilitySlot3`
  (params (Key :type "Key Structure"))
  ;[1 1 1] Roll
  (:`Pressed`
    (`self.Roll`)))

(event `DiveAttack`
  ;[1 1 1] Attacks
  ;;[1 1 1] Dive Attack
  (`self.Can Attack Check`)
  (bind _notifyname (`|PlayMontage` (`self.Skeletal Mesh`) "/Game/Animations/SwordnShield/Mannequin_RM/DiveAttack.DiveAttack")
    (:`then`
      (set `self.IsAttacking` true)
      (`self.ReduceStamina` 25.0)
      (`self.Rotation Correction`))
    (:`OnInterrupted`
      (set `self.IsAttacking` false :!label _label_4))
    (:`OnNotifyBegin`
      (if (== _notifyname "CanAttack")
        (goto _label_4)))))

(event `InputAction|AbilitySlot4`
  (params (Key :type "Key Structure"))
  ;[1 1 1] Attacks
  ;;[1 1 1] Dive Attack
  (:`Pressed`
    (`self.DiveAttack`)))

(event `InputAction|LevelUp Menu`
  (params (Key :type "Key Structure"))
  ;[1 1 1] Show Level Up Menu
  (:`Pressed`
    (`/Engine/EditorBlueprintResources/StandardMacros.FlipFlop`
      (:`A`
        (`self.Show Level Up Menu` true))
      (:`B`
        (`self.Show Level Up Menu` false)))))

(fn `DamageCaluculation`
  (params (Attacker :type "Actor Object Reference") (DamageMultiplayer :type "Float (double-precision)" :default 1.0))
  (bind _returnvalue (`Actor.GetComponentByClass` Attacker "BPC_Combat_C"))
  (set `self.CurrentHealth` (- (`self.CurrentHealth`) (* (* (`/Game/Blueprints/Components/General/BPC_Combat.Damage` _returnvalue) (/ (`/Game/Blueprints/Components/General/BPC_Combat.ATK` _returnvalue) (`self.DEF`))) DamageMultiplayer))))

(fn `DamageEffects`
  (params (`FrameFreeze?` :type Boolean) (Attacker :type "Actor Object Reference"))
  (if `FrameFreeze?`
    (`self.FrameFreeze`))
  (if (== Attacker (`GameplayStatics.GetPlayerCharacter` 0))
    (`PlayerCameraManager.StartCameraShake` :`self` (`GameplayStatics.GetPlayerCameraManager` 0) :`ShakeClass` "/Game/Effects/Camera/CS_Attack.CS_Attack_C")))

(fn `DeathCheck`
  (params (Attacker :type "Actor Object Reference"))
  (if (<= (`self.CurrentHealth`) 0.0)
    (`self.Die` Attacker)))

(fn `FrameFreeze`
  (`GameplayStatics.SetGlobalTimeDilation` 0.05)
  (`KismetSystemLibrary.K2_SetTimer` null "ResetTimeDilation" 0.01))

(fn `IsEnemy`
  (params (Actor :type "Actor Object Reference"))
  (returns (`IsEnemy?` :type Boolean))
  (return (not (== (`/Game/Blueprints/Components/General/BPC_Combat.Team` (`Actor.GetComponentByClass` Actor "BPC_Combat_C")) (`self.Team`)))))

(fn `NewFunction_0`
  (set `self.CurrentStamina` (`KismetMathLibrary.FClamp` (+ (`self.CurrentStamina`) (`self.StaminaRegenSpeed`)) 0.0 (`self.MaxStamina`))))

(fn `ReduceStamina`
  (params (Amount :type "Float (double-precision)"))
  (if (== (`self.GetOwner`) (`GameplayStatics.GetPlayerCharacter` 0))
    (set `self.CurrentStamina` (`KismetMathLibrary.FClamp` (- (`self.CurrentStamina`) Amount) 0.0 (`self.MaxStamina`)))))

(fn `ResetTimeDilation`
  (`GameplayStatics.SetGlobalTimeDilation` 1.0))

(fn `SetRootmotionMode`
  (params (Value :type "ERootMotionMode Enum" :default "RootMotionFromMontagesOnly"))
  (`AnimInstance.SetRootMotionMode` (`SkeletalMeshComponent.GetAnimInstance` (`self.Skeletal Mesh`)) Value))

(fn `Show Level Up Menu`
  (params (`Show?` :type Boolean))
  (if `Show?`
    (bind _returnvalue (`|CreateWidget` "/Game/UI/Widgets/LevelUp/UI_LevelUp.UI_LevelUp_C"))
    (bind _output_get (set `self.LevelUpMenu` _returnvalue))
    (`UserWidget.AddToViewport` _output_get 0)
    (else
      (bind _levelupmenu (`self.LevelUpMenu`)
        (:`then`
          (`Widget.RemoveFromParent` _levelupmenu))
        (:`else`)))))

(fn `UpdateCurrentWeaponData`
  (params (Damage :type "Float (double-precision)") (Mesh :type "StaticMesh Object Reference") (AttachSocket :type Name) (HandSocket :type Name) (OverlayState :type "/Game/AdvancedLocomotionV4/Data/Enums/ALS_OverlayState Enum" :default "NewEnumerator0"))
  (set `self.Damage` Damage)
  (set `self.Mesh` Mesh)
  (set `self.Attach Socket` AttachSocket)
  (set `self.Hand Socket` HandSocket)
  (set `self.Overlay State` OverlayState)
  (`self.WeaponVisuals`))

(fn `WeaponVisuals`
  (bind _weapon_mesh (`self.Weapon Mesh`))
  (`StaticMeshComponent.SetStaticMesh` _weapon_mesh (`self.Mesh`))
  (`SceneComponent.K2_AttachToComponent` _weapon_mesh (`self.Skeletal Mesh`) (`self.Attach Socket`) "SnapToTarget" "SnapToTarget" "SnapToTarget" true))