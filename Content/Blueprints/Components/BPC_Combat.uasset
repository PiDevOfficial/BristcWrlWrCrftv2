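; BPC_Combat is a combat component that holds the owner's current weapon data and displays the weapon on its skeletal mesh.
; An Initialization event stores the skeletal mesh and weapon mesh references.
; UpdateCurrentWeaponData saves damage, mesh and socket names, then calls WeaponVisuals to set the static mesh and snap-attach it to the attach socket.
; Damage and the hand socket are only stored here.
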(event `Initialization`
  (params (SkeletalMesh :type "SkeletalMeshComponent Object Reference") (WeaponMesh :type "StaticMeshComponent Object Reference"))
  (set `self.Skeletal Mesh` SkeletalMesh)
  (set `self.Weapon Mesh` WeaponMesh))

(fn `UpdateCurrentWeaponData`
  (params (Damage :type "Float (double-precision)") (Mesh :type "StaticMesh Object Reference") (AttachSocket :type Name) (HandSocket :type Name))
  (set `self.Damage` Damage)
  (set `self.Mesh` Mesh)
  (set `self.Attach Socket` AttachSocket)
  (set `self.Hand Socket` HandSocket)
  (`self.WeaponVisuals`))

(fn `WeaponVisuals`
  (bind _weapon_mesh (`self.Weapon Mesh`))
  (`StaticMeshComponent.SetStaticMesh` _weapon_mesh (`self.Mesh`))
  (`SceneComponent.K2_AttachToComponent` _weapon_mesh (`self.Skeletal Mesh`) (`self.Attach Socket`) "SnapToTarget" "SnapToTarget" "SnapToTarget" true))